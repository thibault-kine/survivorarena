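; BP_Enemy_Snake is an enemy meant to weave toward the player, damaging BP_Player on overlap.
; Tick applies an unswept offset: a time-based sine on X, not scaled by delta time, and Y from Déplacements, whose chase math appears unconnected.
; TakeDamage lowers health and destroys the actor at zero or below.
; On destruction, it randomly spawns a coin pickup and awards the player points.
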(event Custom|Take%20Damage
  (params (Amount :type Integer))
  ;[0.15 0.15 0.15 0.5] Quand l'ennemi prends des dégâts
  (bind _output_get (Variables|Default|SetHealth_0 (- (Variables|Default|GetHealth_0) Amount)))
  (if (<= _output_get 0)
    (Actor|DestroyActor)))

(event Collision|EventActorBeginOverlap
  (params (OtherActor :type Actor%20Object%20Reference))
  ;[0.15 0.15 0.15 0.5] Au contact du joueur, ce dernier prends des dégâts
  (bind _asbp_player (Utilities|Casting|CastToBP_Player OtherActor))
  (Default|TakeDamage _asbp_player (Variables|Default|GetDamage_0)))

(event EventTick
  (params (DeltaSeconds :type Float%20%28single-precision%29))
  ;[0.15 0.15 0.15 0.5] L'ennemi se déplace vers le joueur
  (Transformation|AddActorWorldOffset (Math|Vector|NegateVector (Math|Vector|MakeVector (* (Math|Trig|Sin(Radians) (Utilities|Time|GetGameTimeinSeconds)) 1.5e+02) (.ReturnValue_Y (|Déplacements DeltaSeconds)) 0.0))))

(event EventDestroyed
  ;[0.15 0.15 0.15 0.5] A la mort de l'ennemi
  (if (Math|Random|RandomBool)
    (Game|SpawnActorfromClass "/Game/Core/Blueprints/BP_CoinPickup.BP_CoinPickup_C" (Transformation|GetActorTransform) "Undefined" "MultiplyWithRoot" 0 0))
  (bind _asbp_player (Utilities|Casting|CastToBP_Player (Game|GetPlayerCharacter 0)))
  (Default|AddPoints _asbp_player (Variables|Default|GetPointsReward_0)))

(fn ConstructionScript)
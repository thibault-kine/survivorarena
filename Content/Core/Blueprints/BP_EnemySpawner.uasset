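; BP_EnemySpawner is a one-shot spawn marker that creates a single enemy at its own position.
; Each tick, it pulses its PaperSprite's scale with a sine of game time, driven by speed, amplitude and base scale variables.
; After a delay from BeginPlay, it spawns BP_EnemyPawn at its X/Y and a fixed height, ignoring collisions, then destroys itself.
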(event EventBeginPlay
  (bind _returnvalue (Transformation|GetActorTransform))
  ;[0.15 0.15 0.15 0.5] Spawn d'ennemi
  (Utilities|FlowControl|Delay (Variables|Default|GetSpawnDelay))
  (Game|SpawnActorfromClass "/Game/Core/Blueprints/BP_EnemyPawn.BP_EnemyPawn_C" (Math|Transform|MakeTransform (Math|Vector|MakeVector (.x (.location _returnvalue)) (.y (.location _returnvalue)) 9e+01) "0, 0, 0" "1.000000,1.000000,1.000000") "AlwaysSpawn" "MultiplyWithRoot" 0 0)
  (Actor|DestroyActor))

(event Collision|EventActorBeginOverlap
  (params (OtherActor :type Actor%20Object%20Reference)))

(event EventTick
  (params (DeltaSeconds :type Float%20%28single-precision%29))
  ;[0.15 0.15 0.15 0.5] Cycle d'animation
  (Transformation|SetWorldScale3D (Variables|Default|GetPaperSprite) (Math|Conversions|ToVector(Float) (+ (* (Math|Trig|Sin(Radians) (* (Utilities|Time|GetGameTimeinSeconds) (Variables|Default|GetScaleSpeed))) (Variables|Default|GetScaleAmp)) (Variables|Default|GetBaseScale)))))

(fn ConstructionScript)
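; Projectile actor that damages a BP_EnemyPawn when its sphere begins overlapping one, then destroys itself.
; CalculateDamage adds BaseDamage to the min and max bounds, rolls a random value between them and applies CritFactor on a CritRate chance.
; Each hit spawns a BP_FloatingText at the projectile's location showing the damage and carrying the crit flag.
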(event OnComponentBeginOverlap(Sphere)
  (params (OverlappedComponent :type Primitive%20Component%20Object%20Reference) (OtherActor :type Actor%20Object%20Reference) (OtherComp :type Primitive%20Component%20Object%20Reference) (OtherBodyIndex :type Integer) (bFromSweep :type Boolean) (SweepResult :type Hit%20Result%20Structure%20%28by%20ref%29))
  ;[0.15 0.15 0.15 0.5] Quand le projectile touche un ennemi
  (bind _asbp_enemy_pawn (Utilities|Casting|CastToBP_EnemyPawn OtherActor))
  (bind (_final_damage _iscrit) (CallFunction|CalculateDamage))
  (bind _output_get (Variables|Damage|SetDamage _final_damage))
  (Default|TakeDamage _asbp_enemy_pawn _output_get)
  ;;[0.15 0.15 0.15 0.5] Spawn Floating Text
  (bind _returnvalue (Game|SpawnActorfromClass "/Game/Core/UI/BP_FloatingText.BP_FloatingText_C" (Math|Transform|MakeTransform (Transformation|GetActorLocation) "0, 0, 0" "1.000000,1.000000,1.000000") "Undefined" "MultiplyWithRoot" 0 0))
  (Variables|/Game/Core/UI/BP_FloatingText.BP_FloatingText_C|SetIsCrit _returnvalue _iscrit)
  (Rendering|Components|TextRender|SetText (Variables|/Game/Core/UI/BP_FloatingText.BP_FloatingText_C|GetTextRender _returnvalue) (Utilities|Text|ToText(Integer) (Variables|Damage|GetDamage)))
  (Actor|DestroyActor))

(event EventBeginPlay)

(event EventTick
  (params (DeltaSeconds :type Float%20%28single-precision%29)))

(fn ConstructionScript
  (Variables|Damage|SetDamage (+ (Variables|Damage|GetDamage) (Variables|Dégâts|GetBaseDamage))))

(fn CalculateDamage
  (bind _output_get (Variables|Dégâts|SetMinDamage (+ (Variables|Dégâts|GetMinDamage) (Variables|Dégâts|GetBaseDamage))))
  (bind _output_get_2 (Variables|Dégâts|SetMaxDamage (+ (Variables|Dégâts|GetMaxDamage) (Variables|Dégâts|GetBaseDamage))))
  (LocalVariables|SetDamageDealt (Math|Random|RandomFloatinRange (Math|Conversions|ToFloat(Integer) _output_get) (Math|Conversions|ToFloat(Integer) _output_get_2)))
  (if (<= (Math|Random|RandomFloatinRange 0.0 1.0) (Variables|Crit|GetCritRate))
    (return (Math|Float|Truncate (* (LocalVariables|GetDamageDealt) (Variables|Crit|GetCritFactor))) true)
    (else
      (return (Math|Float|Truncate (LocalVariables|GetDamageDealt)) false))))
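; Player Blueprint for an auto-firing shooter with experience levels, Enhanced Input movement and clamped camera zoom.
; Tick finds an enemy via sphere overlap (the first in range, not necessarily the closest) and fires projectiles at it, throttled by a Delay.
; Experience from AddPoints raises the level against a growing cap, checked only after firing.
; TakeDamage reduces health, then grants brief invincibility.
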(event Custom|Take%20Damage
  (params (Amount :type Integer))
  ;[0.15 0.15 0.15 0.5] Prendre des dégâts
  (if (Variables|Default|GetCanBeHurt)
    (Variables|Default|SetHealth (- (Variables|Default|GetHealth) Amount))
    (Variables|Default|SetCanBeHurt false)
    (Utilities|FlowControl|Delay (Variables|Default|GetInvincibleTime))
    (Variables|Default|SetCanBeHurt true)))

(event Custom|Add%20Points
  (params (Amount :type Integer))
  ;[0.15 0.15 0.15 0.5] Ajout de points (placeholder)
  (Variables|Default|SetExp (+ Amount (Variables|Default|GetExp))))

(event Input|EnhancedActionEvents|EnhancedInputActionINP_Zoom
  (params (ActionValue :type Float%20%28double-precision%29) (ElapsedSeconds :type Float%20%28double-precision%29) (TriggeredSeconds :type Float%20%28double-precision%29) (InputAction :type Input%20Action%20Object%20Reference :default "/Game/Core/Inputs/INP_Zoom.INP_Zoom"))
  (bind _selfiestick (Variables|Composants|GetSelfieStick))
  ;[0.15 0.15 0.15 0.5] Caméra
  (Variables|Default|SetNewLength (+ ActionValue (Variables|/Script/Engine.SpringArmComponent|GetTargetArmLength _selfiestick)))
  (if (and (<= (Variables|Default|GetNewLength) (Variables|Default|GetMaxZoom)) (>= (Variables|Default|GetNewLength) (Variables|Default|GetMinZoom)))
    (Variables|/Script/Engine.SpringArmComponent|SetTargetArmLength _selfiestick (Variables|Default|GetNewLength))))

(event Input|EnhancedActionEvents|EnhancedInputActionINP_Move
  (params (ActionValue :type Vector%202D%20Structure) (ElapsedSeconds :type Float%20%28double-precision%29) (TriggeredSeconds :type Float%20%28double-precision%29) (InputAction :type Input%20Action%20Object%20Reference :default "/Game/Core/Inputs/INP_Move.INP_Move"))
  ;[0.15 0.15 0.15 0.5] Mouvement
  (Pawn|Input|AddMovementInput (Math|Vector|MakeVector (.x ActionValue) (.y ActionValue) 0.0) 1.0 false))

(event EventTick
  (params (DeltaSeconds :type Float%20%28single-precision%29))
  ;[0.15 0.15 0.15 0.5] On check si des ennemis sont proches
  (bind _enemy (CallFunction|GetClosestEnemy))
  (bind _output_get (Variables|Default|SetClosestEnemy _enemy))
  (Utilities|FlowControl|Delay (Variables|Default|GetFireDelay))
  (Utilities|IsValid _output_get
    (:Is%20Valid
      (CallFunction|FireProjectile "/Game/Core/Blueprints/BP_Projectile.BP_Projectile_C" (Transformation|GetActorLocation _output_get))
      ;[0.15 0.15 0.15 0.5] Gestion de montée de niveau
      (CallFunction|PointsHandler))))

(event Collision|EventActorBeginOverlap
  (params (OtherActor :type Actor%20Object%20Reference)))

(event EventBeginPlay
  ;[0.15 0.15 0.15 0.5] Définit la config des touches par défaut du jeu
  (Input|AddMappingContext (PlayerController|LocalPlayerSubsystems|GetEnhancedInputLocalPlayerSubsystem (Game|GetPlayerController 0)) "/Game/Core/Inputs/IMC_Default.IMC_Default" 0 "(bIgnoreAllPressedKeysUntilRelease=True,bForceImmediately=False,bNotifyUserSettings=False)"))

(fn ConstructionScript)

(fn PointsHandler
  (if (>= (Variables|Default|GetExp) (Variables|Default|GetNextLevelCap))
    (Math|Integer|IncrementInt (Variables|Default|GetLevel)
      (:%20%20
        (Variables|Default|SetNextLevelCap (Math|Float|Floor (* (Math|Conversions|ToFloat(Integer) (Variables|Default|GetNextLevelCap)) 1.5)))
        (Variables|Default|SetExp 0)))))

(fn FireProjectile
  (params (Projectile%20Class :type BP%20Projectile%20Class%20Reference) (Target%20Location :type Vector))
  (bind _self self)
  (bind _returnvalue (Transformation|GetActorLocation _self))
  (Game|SpawnActorfromClass Projectile%20Class (Math|Transform|MakeTransform _returnvalue (Math|Rotator|FindLookatRotation _returnvalue Target%20Location) "1.000000,1.000000,1.000000") "AlwaysSpawn" "MultiplyWithRoot" 0 0))

(fn GetClosestEnemy
  (bind _outactors (Collision|SphereOverlapActors (Transformation|GetActorLocation) (Variables|Default|GetFireRange) (Utilities|Array|MakeArray "ObjectTypeQuery8") "/Game/Core/Blueprints/BP_EnemyPawn.BP_EnemyPawn_C"))
  (for _array_element _outactors
    (bind _asbp_enemy_pawn (Utilities|Casting|CastToBP_EnemyPawn _array_element))
    (if (< (Math|Vector|Distance(Vector) (Transformation|GetActorLocation) (Transformation|GetActorLocation _asbp_enemy_pawn)) (Variables|Default|GetFireRange))
      (return _asbp_enemy_pawn))))
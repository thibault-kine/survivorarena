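; BP_EnemySpawn is a temporary spawn-point actor that shows a pulsing sprite before an enemy appears.
; On BeginPlay it waits for SpawnDelay, spawns BP_Enemy at its own transform regardless of collisions, then destroys itself.
; Meanwhile, Tick animates the PaperSprite's uniform world scale with a sine of game time, driven by speed, amplitude and base-scale variables.
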(event EventBeginPlay
  ;[0.15 0.15 0.15 0.5] Spawn d'ennemi
  (Utilities|FlowControl|Delay (Variables|Default|GetSpawnDelay))
  (Game|SpawnActorfromClass "/Game/Core/Blueprints/BP_Enemy.BP_Enemy_C" (Transformation|GetActorTransform) "AlwaysSpawn" "MultiplyWithRoot" 0 0)
  (Actor|DestroyActor))

(event Collision|EventActorBeginOverlap
  (params (OtherActor :type Actor%20Object%20Reference)))

(event EventTick
  (params (DeltaSeconds :type Float%20%28single-precision%29))
  ;[0.15 0.15 0.15 0.5] Cycle d'animation
  (Transformation|SetWorldScale3D (Variables|Default|GetPaperSprite) (Math|Conversions|ToVector(Float) (+ (* (Math|Trig|Sin(Radians) (* (Utilities|Time|GetGameTimeinSeconds) (Variables|Default|GetScaleSpeed))) (Variables|Default|GetScaleAmp)) (Variables|Default|GetBaseScale)))))

(fn ConstructionScript)